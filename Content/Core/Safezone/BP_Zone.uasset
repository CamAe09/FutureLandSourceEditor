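; BP_Zone is a safe zone that shrinks in timed stages over a match.
; On authority, BeginPlay runs a delay chain of events that lower TargetSize by mostly decreasing steps.
; Tick slowly interpolates the zone mesh's uniform scale toward that target with FInterpTo.
; Mesh overlaps set the character's outside-zone flag on authority and, without an authority check, toggle its post-process and adjust the HUD's ZoneIn counter.
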(event OnComponentBeginOverlap(SM_Zone)
  (params (OverlappedComponent :type Primitive%20Component%20Object%20Reference) (OtherActor :type Actor%20Object%20Reference) (OtherComp :type Primitive%20Component%20Object%20Reference) (OtherBodyIndex :type Integer) (bFromSweep :type Boolean) (SweepResult :type Hit%20Result%20Structure%20%28by%20ref%29))
  (CallFunction|HandleZoneLogic OtherActor false)
  (bind _asbp_crosshair_character (Utilities|Casting|CastToBP_CrosshairCharacter OtherActor))
  (Rendering|SetVisibility (Variables|/Game/CT_Components/Demos/Demo_CrosshairSystem/ThirdPerson/BP_CrosshairCharacter.BP_CrosshairCharacter_C|GetPostProcess _asbp_crosshair_character) false false)
  (Variables|/Game/Core/Widgets/WP_FutureLandHud.WP_FutureLandHud_C|SetZoneIn? (Variables|Default|GetHUD) (- (Variables|/Game/Core/Widgets/WP_FutureLandHud.WP_FutureLandHud_C|GetZoneIn? (Variables|Default|GetHUD)) 1)))

(event OnComponentEndOverlap(SM_Zone)
  (params (OverlappedComponent :type Primitive%20Component%20Object%20Reference) (OtherActor :type Actor%20Object%20Reference) (OtherComp :type Primitive%20Component%20Object%20Reference) (OtherBodyIndex :type Integer))
  (CallFunction|HandleZoneLogic OtherActor true)
  (bind _asbp_crosshair_character (Utilities|Casting|CastToBP_CrosshairCharacter OtherActor))
  (Rendering|SetVisibility (Variables|/Game/CT_Components/Demos/Demo_CrosshairSystem/ThirdPerson/BP_CrosshairCharacter.BP_CrosshairCharacter_C|GetPostProcess _asbp_crosshair_character) true false)
  (Variables|/Game/Core/Widgets/WP_FutureLandHud.WP_FutureLandHud_C|SetZoneIn? (Variables|Default|GetHUD) (+ (Variables|/Game/Core/Widgets/WP_FutureLandHud.WP_FutureLandHud_C|GetZoneIn? (Variables|Default|GetHUD)) 1)))

(event Custom|CustomEvent_7
  (Variables|Default|SetTargetSize (Math|Float|Clamp(Float) (- (.x (Transformation|GetWorldScale (Variables|Default|GetSM_Zone))) 1.0) 0.0 1e+03)))

(event Custom|CustomEvent
  (Variables|Default|SetTargetSize (Math|Float|Clamp(Float) (- (.x (Transformation|GetWorldScale (Variables|Default|GetSM_Zone))) 1.5e+02) 0.0 1e+03)))

(event Custom|CustomEvent_1
  (Variables|Default|SetTargetSize (Math|Float|Clamp(Float) (- (.x (Transformation|GetWorldScale (Variables|Default|GetSM_Zone))) 75.0) 0.0 1e+03)))

(event Custom|CustomEvent_2
  (Variables|Default|SetTargetSize (Math|Float|Clamp(Float) (- (.x (Transformation|GetWorldScale (Variables|Default|GetSM_Zone))) 45.0) 0.0 1e+03)))

(event Custom|CustomEvent_3
  (Variables|Default|SetTargetSize (Math|Float|Clamp(Float) (- (.x (Transformation|GetWorldScale (Variables|Default|GetSM_Zone))) 3e+01) 0.0 1e+03)))

(event Custom|CustomEvent_4
  (Variables|Default|SetTargetSize (Math|Float|Clamp(Float) (- (.x (Transformation|GetWorldScale (Variables|Default|GetSM_Zone))) 25.0) 0.0 1e+03)))

(event Custom|CustomEvent_5
  (Variables|Default|SetTargetSize (Math|Float|Clamp(Float) (- (.x (Transformation|GetWorldScale (Variables|Default|GetSM_Zone))) 25.0) 0.0 1e+03)))

(event Custom|CustomEvent_6
  (Variables|Default|SetTargetSize (Math|Float|Clamp(Float) (- (.x (Transformation|GetWorldScale (Variables|Default|GetSM_Zone))) 15.0) 0.0 1e+03)))

(event Custom|Shrink
  (Variables|Default|SetTargetSize (Math|Float|Clamp(Float) (- (.x (Transformation|GetWorldScale (Variables|Default|GetSM_Zone))) 3.5e+02) 0.0 1e+03)))

(event EventBeginPlay
  (Networking|SwitchHasAuthority
    (:Authority
      (Variables|Default|SetTargetSize (.x (Transformation|GetWorldScale (Variables|Default|GetSM_Zone))))
      (Utilities|FlowControl|Delay 1.0)
      (CallFunction|Shrink)
      (Utilities|FlowControl|Delay 9e+01)
      (CallFunction|CustomEvent)
      (Utilities|FlowControl|Delay 7e+01)
      (CallFunction|CustomEvent1)
      (Utilities|FlowControl|Delay 6e+01)
      (CallFunction|CustomEvent2)
      (Utilities|FlowControl|Delay 6e+01)
      (CallFunction|CustomEvent3)
      (Utilities|FlowControl|Delay 45.0)
      (CallFunction|CustomEvent4)
      (Utilities|FlowControl|Delay 4e+01)
      (CallFunction|CustomEvent5)
      (Utilities|FlowControl|Delay 35.0)
      (CallFunction|CustomEvent6)
      (Utilities|FlowControl|Delay 35.0)
      (CallFunction|CustomEvent7))))

(event EventTick
  (params (DeltaSeconds :type Float%20%28single-precision%29))
  (bind _targetsize (Variables|Default|GetTargetSize))
  (bind _sm_zone (Variables|Default|GetSM_Zone))
  (bind _returnvalue (Transformation|GetWorldScale _sm_zone))
  (bind _returnvalue_2 (Math|Interpolation|FInterpTo (.x _returnvalue) _targetsize DeltaSeconds 0.01))
  (if (not (== (.x _returnvalue) 0.0))
    (Transformation|SetWorldScale3D (Variables|Default|GetSM_Zone) (Math|Vector|MakeVector _returnvalue_2 _returnvalue_2 _returnvalue_2))))

(fn ConstructionScript)

(fn HandleZoneLogic
  (params (OtherActor :type Object%20Object%20Reference) (OutsideZone? :type Boolean))
  (Networking|SwitchHasAuthority
    (:Authority
      (if (== (Utilities|GetClass OtherActor) "/Game/CT_Components/Demos/Demo_CrosshairSystem/ThirdPerson/BP_CrosshairCharacter.BP_CrosshairCharacter_C")
        (bind _asbp_crosshair_character (Utilities|Casting|CastToBP_CrosshairCharacter OtherActor))
        (Variables|/Game/CT_Components/Demos/Demo_CrosshairSystem/ThirdPerson/BP_CrosshairCharacter.BP_CrosshairCharacter_C|SetIsoutsidezone _asbp_crosshair_character OutsideZone?)))))