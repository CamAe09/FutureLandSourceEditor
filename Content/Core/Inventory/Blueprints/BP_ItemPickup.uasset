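; BP_ItemPickup is a world pickup actor that displays a weapon until it is interacted with.
; On BeginPlay it spawns the Blueprint class from its Weapon data at the Arrow component's location, keeps a reference, and turns off shadow casting on that actor's skeletal mesh.
; The Interaction event destroys both the pickup and the spawned weapon, with no inventory transfer in this graph.
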(event EventBeginPlay
  (bind _returnvalue (Game|SpawnActorfromClass (Variables|/Game/Core/Weapons/WeaponIdentitys/BP_WeaponIdentity.BP_WeaponIdentity_C|GetWeapon%20Blueprint (Variables|Default|GetWeapon)) (Math|Transform|MakeTransform (Transformation|GetWorldLocation (Variables|Default|GetArrow)) "0, 0, 0" "1.000000,1.000000,1.000000") "Undefined" "MultiplyWithRoot" self 0.0 0))
  (Variables|Default|SetWeapon%20Actor%20Ref _returnvalue)
  (Rendering|SetCastShadow (Variables|/Game/Core/Weapons/WeaponBlueprints/BP_WeaponBase.BP_WeaponBase_C|GetSkeletalMesh _returnvalue) false))

(event EventInteraction
  (Actor|DestroyActor)
  (Actor|DestroyActor (Variables|Default|GetWeapon%20Actor%20Ref)))

(fn ConstructionScript)